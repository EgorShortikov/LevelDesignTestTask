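; A machine gun turret that tracks the player's third-person character and shoots projectiles at it when in range.
; Each Tick turns MachinegunFoot toward the player using a look-at rotation, remapping pitch to roll and offsetting yaw for the mesh orientation.
; A Delay in Tick throttles firing, which spawns BP_Projectile at the Arrow with a shot sound whenever the player is within the Sphere's radius.
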(event EventBeginPlay
  (bind _asbp_third_person_character (Utilities|Casting|CastToBP_ThirdPersonCharacter (Game|Player|GetPlayerPawn 0)))
  (Variables|Default|SetThird%20Person%20Character _asbp_third_person_character))

(event EventTick
  (params (DeltaSeconds :type Float%20%28single-precision%29))
  (CallFunction|Rotate)
  (Utilities|FlowControl|Delay 0.2)
  (CallFunction|Fire))

(fn ConstructionScript)

(fn Rotate
  (bind _output_get (Variables|Default|SetPlayerLocation (Transformation|GetActorLocation (Variables|Default|GetThird%20Person%20Character))))
  (bind _output_get_2 (Variables|Default|SetMachinegun%20Location (Transformation|GetWorldLocation (Variables|Default|GetArrow))))
  (Variables|Default|SetReturn%20Value%20Z%20%28Yaw%29 (- (.yaw (Math|Rotator|FindLookatRotation _output_get_2 _output_get)) 9e+01))
  (Transformation|SetWorldRotation (Variables|Default|GetMachinegunFoot) (Math|Rotator|MakeRotator 0.0 0.0 0.0) false false)
  (Transformation|SetWorldRotation (Variables|Default|GetMachinegunFoot) (Math|Rotator|MakeRotator (* (.pitch (Math|Rotator|FindLookatRotation _output_get_2 _output_get)) -1.0) 0.0 (Variables|Default|GetReturn%20Value%20Z%20%28Yaw%29)) false false))

(fn Fire
  (bind _arrow (Variables|Default|GetArrow))
  (bind _returnvalue (Transformation|GetWorldRotation _arrow))
  (if (< (Math|Vector|Distance(Vector) (Variables|Default|GetPlayerLocation) (Variables|Default|GetMachinegun%20Location)) (Variables|/Script/Engine.SphereComponent|GetSphereRadius (Variables|Default|GetSphere)))
    (Game|SpawnActorfromClass "/Game/MachineGun/Blueprints/BP_Projectile.BP_Projectile_C" (Math|Transform|MakeTransform (Transformation|GetWorldLocation _arrow) (Math|Rotator|MakeRotator (.roll _returnvalue) (.pitch _returnvalue) (.yaw _returnvalue)) "1.000000,1.000000,1.000000") "Undefined" "MultiplyWithRoot" 0 0)
    (Audio|PlaySoundatLocation "/Game/MachineGun/Audio/Shoot.Shoot" (Variables|Default|GetMachinegun%20Location) "0, 0, 0" 1.0 1.0 0.0 0 0 0 0)))