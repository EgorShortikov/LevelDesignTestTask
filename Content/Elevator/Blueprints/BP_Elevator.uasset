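; BP_Elevator is a one-shot elevator that starts moving when anything overlaps its Box trigger.
; The overlap destroys the Box, plays a 2D sound, waits briefly, then plays a Timeline.
; Each update offsets the Cube's Z from the height cached at BeginPlay, using the track's Z value.
; The actor's world coordinates are fed into SetRelativeLocation, mixing world and relative space.
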(event OnComponentEndOverlap(Box)
  (params (OverlappedComponent :type Primitive%20Component%20Object%20Reference) (OtherActor :type Actor%20Object%20Reference) (OtherComp :type Primitive%20Component%20Object%20Reference) (OtherBodyIndex :type Integer)))

(event OnComponentBeginOverlap(Box)
  (params (OverlappedComponent :type Primitive%20Component%20Object%20Reference) (OtherActor :type Actor%20Object%20Reference) (OtherComp :type Primitive%20Component%20Object%20Reference) (OtherBodyIndex :type Integer) (bFromSweep :type Boolean) (SweepResult :type Hit%20Result%20Structure%20%28by%20ref%29))
  (bind _returnvalue (Transformation|GetActorLocation))
  (Components|DestroyComponent (Variables|Default|GetBox))
  (Audio|PlaySound2D "/Game/Elevator/Audio/ElevatorGoing.ElevatorGoing" 1.0 1.0 0.0 0 0)
  (Utilities|FlowControl|Delay 0.5)
  (bind _elevatormovement (Timeline|Timeline Play)
    (:Update
      (Transformation|SetRelativeLocation (Variables|Default|GetCube) (Math|Vector|MakeVector (.x _returnvalue) (.y _returnvalue) (+ (.z _elevatormovement) (stale EventBeginPlay _output_get))) false false))))

(event Collision|EventActorBeginOverlap
  (params (OtherActor :type Actor%20Object%20Reference)))

(event EventTick
  (params (DeltaSeconds :type Float%20%28single-precision%29)))

(event EventBeginPlay
  (bind _output_get (Variables|Default|SetElevatorStartZLocation (.z (Transformation|GetActorLocation)))))

(fn ConstructionScript)